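; BP_HoverPlatform is a platform that hovers above surfaces using physics forces on its static mesh.
; Each tick it line-traces a short distance straight down from the mesh for world static and dynamic objects, drawing the trace for debugging.
; On a hit, it pushes the mesh upward with a mass-independent acceleration that grows linearly as the surface gets closer, acting as an undamped spring.
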(event `self.ReceiveTick`
  (params (DeltaSeconds :type "Float (single-precision)"))
  (bind (_outhit _returnvalue) (`KismetSystemLibrary.LineTraceSingleForObjects` :`Start` (`SceneComponent.K2_GetComponentLocation` (`self.StaticMesh`)) :`End` (+ (`SceneComponent.K2_GetComponentLocation` (`self.StaticMesh`)) (0.0 0.0 -350.0)) :`ObjectTypes` (`|MakeArray` "ObjectTypeQuery1" "ObjectTypeQuery2" :!type "EObjectTypeQuery Enum") :`DrawDebugType` "ForOneFrame"))
  (if _returnvalue
    (`PrimitiveComponent.AddForce` (`self.StaticMesh`) (* (0.0 0.0 3000.0) (- 1.0 (`.Time` (`GameplayStatics.BreakHitResult` _outhit)))) "None" true)))

(fn `UserConstructionScript`)